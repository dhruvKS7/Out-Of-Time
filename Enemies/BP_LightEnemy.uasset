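; BP_LightEnemy is a simple Barghest enemy that runs straight ahead and bites when something overlaps its box.
; Tick adds forward movement input while CanMove is set.
; Box overlap begin and end toggle that flag and switch between looping bite and run animations, without filtering the overlapping actor or applying damage.
; Optional tail and mane meshes follow the main Mesh's skeleton via leader pose.
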(event OnComponentBeginOverlap(Box)
  (params (OverlappedComponent :type Primitive%20Component%20Object%20Reference) (OtherActor :type Actor%20Object%20Reference) (OtherComp :type Primitive%20Component%20Object%20Reference) (OtherBodyIndex :type Integer) (bFromSweep :type Boolean) (SweepResult :type Hit%20Result%20Structure%20%28by%20ref%29))
  (Variables|Default|SetcanMove false)
  (Components|Animation|PlayAnimation (Variables|Character|GetMesh) "/Game/QuadrapedCreatures/Barghest/Animations/BARGHEST_biteNormal.BARGHEST_biteNormal" true))

(event OnComponentEndOverlap(Box)
  (params (OverlappedComponent :type Primitive%20Component%20Object%20Reference) (OtherActor :type Actor%20Object%20Reference) (OtherComp :type Primitive%20Component%20Object%20Reference) (OtherBodyIndex :type Integer))
  (Variables|Default|SetcanMove true)
  (Components|Animation|PlayAnimation (Variables|Character|GetMesh) "/Game/QuadrapedCreatures/Barghest/Animations/BARGHEST_run.BARGHEST_run" true))

(event EventBeginPlay
  ;[1 1 1] Make the optional meshes to use the same skeleton as Barghest
  (Components|SkinnedMesh|SetLeaderPoseComponent (Variables|Default|GetBargahest_Tail) (Variables|Character|GetMesh) false false)
  (Components|Animation|PlayAnimation (Variables|Character|GetMesh) "/Game/QuadrapedCreatures/Barghest/Animations/BARGHEST_run.BARGHEST_run" true))

(event Collision|EventActorBeginOverlap
  (params (OtherActor :type Actor%20Object%20Reference)))

(event EventTick
  (params (DeltaSeconds :type Float%20%28single-precision%29))
  (if (Variables|Default|GetcanMove)
    (Pawn|Input|AddMovementInput (Transformation|GetActorForwardVector) 1.0 false)))

(fn ConstructionScript)